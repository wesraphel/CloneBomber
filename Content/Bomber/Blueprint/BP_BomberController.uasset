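; BP_BomberController is the player controller for a local two-player Bomberman game, routing separate move and bomb inputs to player characters 0 and 1.
; Movement uses world axes and also fires Moverfoward/Moverright dispatchers.
; It registers with BP_BomberGM on BeginPlay.
; On possess, it caches the Bomberman and reads TelaCompartilhada from the game instance to choose the game mode's shared camera or a per-player split-screen widget.
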(event `InputAction|Bomba2`
  (params (Key :type "Key Structure"))
  (:`Pressed`
    (bind _asbp_bomberman (cast `/Game/Bomber/BomberPlayer/BP_Bomberman` (`GameplayStatics.GetPlayerCharacter` 1)))
    (`/Game/Bomber/BomberPlayer/BP_Bomberman.ColocarBomba2` _asbp_bomberman)))

(event `InputAxis|MoveRight2`
  (params (AxisValue :type "Float (single-precision)"))
  (bind _asbp_bomberman (cast `/Game/Bomber/BomberPlayer/BP_Bomberman` (`GameplayStatics.GetPlayerCharacter` 1)))
  (`Pawn.AddMovementInput` _asbp_bomberman (1.0 0.0 0.0) AxisValue false)
  (`self.moverfowardevent` AxisValue))

(event `InputAxis|MoveForward2`
  (params (AxisValue :type "Float (single-precision)"))
  (bind _asbp_bomberman (cast `/Game/Bomber/BomberPlayer/BP_Bomberman` (`GameplayStatics.GetPlayerCharacter` 1)))
  (`Pawn.AddMovementInput` _asbp_bomberman (0.0 1.0 0.0) AxisValue false)
  (`self.moverrightevent` AxisValue))

(event `InputAction|Bomba`
  (params (Key :type "Key Structure"))
  (:`Pressed`
    (bind _asbp_bomberman (cast `/Game/Bomber/BomberPlayer/BP_Bomberman` (`GameplayStatics.GetPlayerCharacter` 0)))
    (`/Game/Bomber/BomberPlayer/BP_Bomberman.ColocarBomba1` _asbp_bomberman)))

(event `InputAxis|MoveRight`
  (params (AxisValue :type "Float (single-precision)"))
  (bind _asbp_bomberman (cast `/Game/Bomber/BomberPlayer/BP_Bomberman` (`GameplayStatics.GetPlayerCharacter` 0)))
  (`Pawn.AddMovementInput` _asbp_bomberman (1.0 0.0 0.0) AxisValue false)
  (`self.moverfowardevent` AxisValue))

(event `InputAxis|MoveForward`
  (params (AxisValue :type "Float (single-precision)"))
  (bind _asbp_bomberman (cast `/Game/Bomber/BomberPlayer/BP_Bomberman` (`GameplayStatics.GetPlayerCharacter` 0)))
  (`Pawn.AddMovementInput` _asbp_bomberman (0.0 1.0 0.0) AxisValue false)
  (`self.moverrightevent` AxisValue))

(event `self.ReceiveBeginPlay`
  (bind _asbp_bomber_gm (cast `/Game/Bomber/Blueprint/BP_BomberGM` (`GameplayStatics.GetGameMode`)))
  (bind _output_get (set `self.GM` _asbp_bomber_gm))
  (`/Game/Bomber/Blueprint/BP_BomberGM.ReceberControlador` _output_get self))

(event `self.ReceivePossess`
  (params (PossessedPawn :type "Pawn Object Reference"))
  (`|ExecutionSequence`
    (:`then_0`
      (bind _asbp_bomberman (cast `/Game/Bomber/BomberPlayer/BP_Bomberman` PossessedPawn))
      (set `self.Bomberman` _asbp_bomberman))
    (:`then_1`
      (bind _asbp_bomber_instance (cast `/Game/Bomber/Blueprint/BP_BomberInstance` (`GameplayStatics.GetGameInstance`)))
      (if (not (`/Game/Bomber/Blueprint/BP_BomberInstance.telaCompartilhada` _asbp_bomber_instance))
        (bind _returnvalue (`|CreateWidget` "/Game/Bomber/Widget/WBP_Dividida.WBP_Dividida_C" self))
        (bind _output_get (set `self.WBPDividida` _returnvalue))
        (`UserWidget.AddToPlayerScreen` _output_get 0)
        (else
          (bind _gm (`self.GM`)
            (:`then`
              (`self.SetViewTargetWithBlend` (`/Game/Bomber/Blueprint/BP_BomberGM.CameraPrincipal` _gm)))
            (:`else`)))))))

(event `self.ReceiveUnPossess`
  (params (UnpossessedPawn :type "Pawn Object Reference"))
  (set `self.Bomberman` null))

(fn `UserConstructionScript`)