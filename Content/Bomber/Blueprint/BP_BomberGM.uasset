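; BP_BomberGM is the Bomber game mode, setting up local two-player play and handling the death screen.
; On BeginPlay it applies the game instance's TelaCompartilhada (shared screen) flag, disabling splitscreen and showing a shared-screen widget, and creates player 1.
; ReceberCamera and ReceberControlador store camera and controller, so in shared mode that controller views the camera whichever arrives first.
; Morte pauses the game and opens the death widget with a mouse cursor.
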(event `self.ReceiveBeginPlay`
  (`|ExecutionSequence`
    (:`then_0`
      (bind _asbp_bomber_instance (cast `/Game/Bomber/Blueprint/BP_BomberInstance` (`GameplayStatics.GetGameInstance`)))
      (bind _output_get (set `self.gameInstance` _asbp_bomber_instance))
      (bind _telacompartilhada (`/Game/Bomber/Blueprint/BP_BomberInstance.telaCompartilhada` _output_get))
      (`GameplayStatics.SetForceDisableSplitscreen` _telacompartilhada)
      (if _telacompartilhada
        (bind _returnvalue (`|CreateWidget` "/Game/Bomber/Widget/WBP_Compartilhada.WBP_Compartilhada_C"))
        (bind _output_get_2 (set `self.WBPCompartilhada` _returnvalue))
        (`UserWidget.AddToViewport` _output_get_2 0)))
    (:`then_1`
      (bind _returnvalue_2 (`GameplayStatics.CreatePlayer` 1))
      (bind _asbp_bomber_controller (cast `/Game/Bomber/Blueprint/BP_BomberController` _returnvalue_2))
      (`self.ReceberControlador` _asbp_bomber_controller))))

(event `self.ReceiveTick`
  (params (DeltaSeconds :type "Float (single-precision)")))

(fn `CameraPrincipal`
  (returns (CameraPrincipal :type "/Game/Bomber/Blueprint/BP_Camera Object Reference"))
  (return (`self.camera`)))

(fn `Morte`
  (`GameplayStatics.SetGamePaused` true)
  (bind _returnvalue (`|CreateWidget` "/Game/Bomber/Widget/WBP_Morte.WBP_Morte_C" (`GameplayStatics.GetPlayerController` 0)))
  (bind _output_get (set `self.WBPMorte` _returnvalue))
  (`UserWidget.AddToViewport` _output_get 0)
  (set `PlayerController.bShowMouseCursor` true (`GameplayStatics.GetPlayerController` 0))
  (`/Game/Bomber/Widget/WBP_Morte.ChamarWidget` (`self.WBPMorte`)))

(fn `ReceberCamera`
  (params (Camera :type "/Game/Bomber/Blueprint/BP_Camera Object Reference"))
  (bind _asbp_bomber_instance (cast `/Game/Bomber/Blueprint/BP_BomberInstance` (`GameplayStatics.GetGameInstance`)))
  (set `self.camera` Camera)
  (if (`/Game/Bomber/Blueprint/BP_BomberInstance.telaCompartilhada` _asbp_bomber_instance)
    (`PlayerController.SetViewTargetWithBlend` (`self.playerController`) (`self.camera`) 0.0 "VTBlend_Linear" 0.0 false)))

(fn `ReceberControlador`
  (params (`[0]` :type "/Game/Bomber/Blueprint/BP_BomberController Object Reference"))
  (bind _asbp_bomber_instance (cast `/Game/Bomber/Blueprint/BP_BomberInstance` (`GameplayStatics.GetGameInstance`)))
  (set `self.playerController` (`|MakeArray` `[0]`))
  (`|ExecutionSequence`
    (:`then_0`
      (if (`/Game/Bomber/Blueprint/BP_BomberInstance.telaCompartilhada` _asbp_bomber_instance)
        (bind _camera (`self.camera`)
          (:`then`
            (`PlayerController.SetViewTargetWithBlend` (`self.playerController`) _camera 0.0 "VTBlend_Linear" 0.0 false))
          (:`else`))))))

(fn `UserConstructionScript`)