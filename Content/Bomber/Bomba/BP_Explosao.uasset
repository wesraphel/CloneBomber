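; BP_Explosao is a bomb explosion segment in a Bomberman-style game that kills any Bomberman it touches.
; On spawn it plays the bomb sound and sets its range from the player's Fogo stat, then travels forward until that range and destroys itself after a short delay.
; While moving, its Box overlap sets Morto and calls Morte on the game mode.
; A forward box trace runs, but its range-clipping logic is disconnected.
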(event `self.ReceiveBeginPlay`
  (bind _posinicial (`self.posInicial`))
  (`|ExecutionSequence`
    (:`then_0`
      (bind _asbp_bomberman (cast `/Game/Bomber/BomberPlayer/BP_Bomberman` (`GameplayStatics.GetPlayerCharacter` 0)))
      (set `self.Bomberman` _asbp_bomberman)
      (bind _asbp_bomber_gm (cast `/Game/Bomber/Blueprint/BP_BomberGM` (`GameplayStatics.GetGameMode`)))
      (set `self.GM` _asbp_bomber_gm))
    (:`then_1`
      (set `self.tam` (* (`/Game/Bomber/BomberPlayer/BP_Bomberman.+Fogo` (`self.Bomberman`)) 4.0))
      (set `self.posInicial` (`self.K2_GetActorLocation`))
      (bind (_outhit _returnvalue) (`KismetSystemLibrary.BoxTraceSingleForObjects` _posinicial (+ _posinicial (* (`self.GetActorForwardVector`) (`self.tam`))) (20.0 20.0 20.0) (struct) (`|MakeArray` "ObjectTypeQuery1" :!type "EObjectTypeQuery Enum")))
      (`GameplayStatics.PlaySoundAtLocation` "/Game/Bomber/Sons/bomba_Cue.bomba_Cue" (`SceneComponent.K2_GetComponentLocation` (`self.Box`)) (struct) 1.0 1.0 0.0 null null null))))

(event `self.ReceiveTick`
  (params (DeltaSeconds :type "Float (single-precision)"))
  (if (not (`self.stop?`))
    (`self.K2_AddActorWorldOffset` (* (`self.GetActorForwardVector`) (* DeltaSeconds (`self.vel`))))
    (if (>= (`KismetMathLibrary.VSize` (- (`self.posInicial`) (`self.K2_GetActorLocation`))) (`self.tam`))
      (set `self.stop?` true)
      (`KismetSystemLibrary.Delay` 0.5)
      (`self.K2_DestroyActor`))))

(event `self.Box.OnComponentBeginOverlap`
  (params (OverlappedComponent :type "PrimitiveComponent Object Reference") (OtherActor :type "Actor Object Reference") (OtherComp :type "PrimitiveComponent Object Reference") (OtherBodyIndex :type Integer) (bFromSweep :type Boolean) (SweepResult :type "HitResult Structure (by ref)"))
  (if (not (`self.stop?`))
    (bind _asbp_bomberman (cast `/Game/Bomber/BomberPlayer/BP_Bomberman` OtherActor))
    (set `/Game/Bomber/BomberPlayer/BP_Bomberman.morto` true _asbp_bomberman)
    (`/Game/Bomber/Blueprint/BP_BomberGM.Morte` (`self.GM`))))

(fn `UserConstructionScript`)