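; BP_Bomba is the bomb actor in a Bomberman-style game.
; On BeginPlay it caches a BP_Bomberman reference from players 0 and 1 in one variable, the second overwriting the first.
; The Timeline_Explosao timeline animates the mesh scale as a fuse.
; When it finishes, Explosão spawns BP_Explosao at AreaExplosão facing the four world axis directions, then destroys the bomb.
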(event `self.ReceiveBeginPlay`
  (bind _staticmesh (`self.StaticMesh`))
  (`|ExecutionSequence`
    (:`then_0`
      (bind _asbp_bomberman (cast `/Game/Bomber/BomberPlayer/BP_Bomberman` (`GameplayStatics.GetPlayerCharacter` 0)))
      (set `self.Bomber` _asbp_bomberman)
      (bind _asbp_bomberman_2 (cast `/Game/Bomber/BomberPlayer/BP_Bomberman` (`GameplayStatics.GetPlayerCharacter` 1)))
      (set `self.Bomber` _asbp_bomberman_2))
    (:`then_1`
      (bind (_direction _tamanho_antes_da_morte) (`Timeline|Timeline_Explosao`)
        (:`Update`
          (`/Engine/EditorBlueprintResources/StandardMacros.IsValid` _staticmesh
            (:`Is Valid`
              (`SceneComponent.SetWorldScale3D` _staticmesh (`KismetMathLibrary.Conv_DoubleToVector` _tamanho_antes_da_morte)))))
        (:`Finished`
          (`self.Explosão`))))))

(fn `Explosão`
  (for _array_element (`|MakeArray` (1.0 0.0 0.0) (0.0 1.0 0.0) (-1.0 0.0 0.0) (0.0 -1.0 0.0) :!type "Vector Structure")
    (`|SpawnActorFromClass` "/Game/Bomber/Bomba/BP_Explosao.BP_Explosao_C" (`KismetMathLibrary.MakeTransform` (`SceneComponent.K2_GetComponentLocation` (`self.areaExplosão`)) (`KismetMathLibrary.Conv_VectorToRotator` _array_element)) "Undefined" "OverrideRootScale" null null))
  (`self.K2_DestroyActor`))

(fn `UserConstructionScript`)