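; BP_CopiaExplosiva is a copy pawn spawned by BP_Bomberman that moves from its owner's player input.
; On BeginPlay it casts its owner to BP_Bomberman and binds to the forward and right move events of that owner's BP_BomberController.
; Both handlers add forced movement along fixed negative world X and Y axes, scaled by MultiplicarVelocidade.
; No explosion logic lives here; the MoveForward function is empty.
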(event `self.ReceiveBeginPlay`
  (`parent.ReceiveBeginPlay`)
  (bind _asbp_bomberman (cast `/Game/Bomber/BomberPlayer/BP_Bomberman` (`self.GetOwner`)))
  (set `/Game/Bomber/BomberPlayer/BP_Bomberman.+Fogo` (`/Game/Bomber/BomberPlayer/BP_Bomberman.+Fogo` _asbp_bomberman) _asbp_bomberman)
  (bind _asbp_bomber_controller (cast `/Game/Bomber/Blueprint/BP_BomberController` (`self.GetController` _asbp_bomberman)))
  (bind _output_get (set `self.playerController` _asbp_bomber_controller))
  (add `/Game/Bomber/Blueprint/BP_BomberController.moverfowardevent` _output_get (delegate `MoveForwardCopiaExplosiva`))
  (add `/Game/Bomber/Blueprint/BP_BomberController.moverrightevent` _output_get (delegate `MoveRightCopiaExplosiva`)))

(event `MoveForwardCopiaExplosiva`
  (params (axisValue :type "Float (double-precision)"))
  (`self.AddMovementInput` (-1.0 0.0 0.0) (* axisValue (`self.multiplicarVelocidade`)) true))

(event `MoveRightCopiaExplosiva`
  (params (axisValue :type "Float (double-precision)"))
  (`self.AddMovementInput` (0.0 -1.0 0.0) (* axisValue (`self.multiplicarVelocidade`)) true))

(fn `MoveForward`)

(fn `UserConstructionScript`
  (`parent.UserConstructionScript`))